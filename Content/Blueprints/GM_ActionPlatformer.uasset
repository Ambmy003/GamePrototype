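; Game mode for an action platformer that handles respawning the player.
; On BeginPlay it finds and caches the level's Player Start.
; RespawnPlayer spawns a fresh default pawn at the active checkpoint's Scene component transform, or at the Player Start when no valid checkpoint exists, and has player controller 0 possess it.
; Spawning always succeeds regardless of collision.
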(event EventBeginPlay
  (bind _returnvalue (Actor|GetActorOfClass "/Script/Engine.PlayerStart"))
  (Variables|Default|SetPlayerStart _returnvalue))

(event EventTick
  (params (DeltaSeconds :type Float%20%28single-precision%29)))

(fn ConstructionScript)

(fn RespawnPlayer
  (bind _playerstart (Variables|Default|GetPlayerStart))
  (bind _activecheckpoint (Variables|Default|GetActiveCheckpoint))
  (bind _returnvalue (Transformation|GetActorTransform _playerstart))
  (bind _scene (Variables|/Game/Blueprints/Props/BP_Checkpoint.BP_Checkpoint_C|GetScene _activecheckpoint))
  (bind _returnvalue_2 (Transformation|GetWorldTransform _scene))
  (Utilities|IsValid (Variables|Default|GetActiveCheckpoint)
    (:Is%20Valid
      ;[1 1 1] Selects Checkpoint If One Is Active and Valid
      (bind _returnvalue_3 (Game|SpawnActorfromClass (Variables|Default|GetDefaultPawnClass) (Math|Transform|MakeTransform (.location _returnvalue_2) (.rotation _returnvalue_2) "1.000000,1.000000,1.000000") "AlwaysSpawn" "MultiplyWithRoot" 0 0))
      (Pawn|Possess (Game|GetPlayerController 0) _returnvalue_3))
    (:Is%20Not%20Valid
      ;[1 1 1] Sends Player To Player Start If No Active Or Valid Checkpoint Exists
      (bind _returnvalue_4 (Game|SpawnActorfromClass (Variables|Default|GetDefaultPawnClass) (Math|Transform|MakeTransform (.location _returnvalue) (.rotation _returnvalue) "1.000000,1.000000,1.000000") "AlwaysSpawn" "MultiplyWithRoot" 0 0))
      (Pawn|Possess (Game|GetPlayerController 0) _returnvalue_4))))