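; AI controller for the cave bat enemy that steers it toward a target player.
; On possess it caches the pawn as a cave bat, and a SetTargetPlayer event supplies the target.
; Each tick, while both references are valid, it calls the bat's MoveTowards with the straight-line direction to the player, using no pathfinding or behavior tree.
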(event Custom|SetTargetPlayer
  (params (TargetPlayer :type Pawn%20Object%20Reference))
  (Variables|Default|SetTargetPlayer TargetPlayer))

(event EventTick
  (params (DeltaSeconds :type Float%20%28single-precision%29))
  (Utilities|IsValid (Variables|Default|GetOwningCaveBat)
    (:Is%20Valid
      (Utilities|IsValid (Variables|Default|GetTargetPlayer)
        (:Is%20Valid
          (Default|MoveTowards (Variables|Default|GetOwningCaveBat) (Math|Vector|GetForwardVector (Math|Rotator|FindLookatRotation (Transformation|GetActorLocation (Variables|Default|GetOwningCaveBat)) (Transformation|GetActorLocation (Variables|Default|GetTargetPlayer)))) 1.0))))))

(event EventPossess
  (params (PossessedPawn :type Pawn%20Object%20Reference))
  (bind _asbp_enemy_cave_bat (Utilities|Casting|CastToBP_Enemy_CaveBat PossessedPawn))
  (Variables|Default|SetOwningCaveBat _asbp_enemy_cave_bat))

(fn ConstructionScript
  (|CallParentFunction))