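; Player character for a 2D action platformer with movement, wall slide and jump, energy-limited charge shooting, and death respawn through the game mode.
; Enhanced Input drives actions, while Tick runs wall traces and eases the spring arm toward the player or an overlapping camera restrictor.
; Damage updates the HUD, cancels charging, and triggers knockback, stun and flickering invincibility.
; BeginPlay builds parallax background materials; ground slide is mostly disabled, optional wiring.
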(event OnComponentBeginOverlap(CapsuleComponent)
  (params (OverlappedComponent :type Primitive%20Component%20Object%20Reference) (OtherActor :type Actor%20Object%20Reference) (OtherComp :type Primitive%20Component%20Object%20Reference) (OtherBodyIndex :type Integer) (bFromSweep :type Boolean) (SweepResult :type Hit%20Result%20Structure%20%28by%20ref%29))
  ;[1 1 1] Player Character Damage (Touching Enemy)
  (bind _asbp_enemy_base (Utilities|Casting|CastToBP_Enemy_BASE OtherActor))
  (if (== (Variables|/Script/Engine.Character|GetCapsuleComponent _asbp_enemy_base) OtherComp)
    (Game|Damage|ApplyDamage self (Variables|Vitality|GetOverlapDamage) 0 _asbp_enemy_base)))

(event Custom|TriggerInvincibility
  ;[1 1 1] Damage Flicker and Invicibility
  (Collision|SetCollisionResponsetoChannel (Variables|Default|GetCapsuleComponent) "ECC_Pawn" "ECR_Ignore")
  (bind _returnvalue (Utilities|Time|SetTimerbyEvent (EventDispatchers|CreateEvent :!event ToggleSpriteFlicker) (Variables|Vitality|GetSpriteFlickerInterval) true))
  (Variables|Vitality|SetFlickerHandle _returnvalue)
  (Utilities|FlowControl|RetriggerableDelay (Variables|Vitality|GetInvincibilityDuration))
  (Utilities|Time|ClearandInvalidateTimerbyHandle (Variables|Vitality|GetFlickerHandle))
  (Collision|SetCollisionResponsetoChannel (Variables|Default|GetCapsuleComponent) "ECC_Pawn" "ECR_Overlap")
  (Rendering|SetVisibility (Variables|Default|GetSprite) true true))

(event Custom|TriggerShootAnim
  ;[1 1 1] Trigger Shoot Anim Event Logic
  (Variables|Shooting|SetIsShooting true)
  (Utilities|FlowControl|RetriggerableDelay (Variables|Shooting|GetShootAnimDuration))
  (Variables|Shooting|SetIsShooting false))

(event Custom|Cancel%20Slide
  ;[1 1 1] Slide Mechanics (Connect To Jump and Wall Jumping If Wanting To Slide - ACTIVATE OTHER DISABLED NODES ON GRAPH IF WANTING TO USE SLIDE)
  (Utilities|IsValid (stale _asynctaskproxy)
    (:Is%20Valid
      (AsyncAction|Cancel (stale _asynctaskproxy))
      (Variables|Slide|SetIsGroundSliding false))))

(event Custom|OnDefeated
  ;[1 1 1] Control Mapping
  ;;[1 1 1] Player Respawn
  (|RespawnSequence))

(event Input|EnhancedActionEvents|EnhancedInputActionIA_Jump
  (params (ActionValue :type Boolean) (ElapsedSeconds :type Float%20%28double-precision%29) (TriggeredSeconds :type Float%20%28double-precision%29) (InputAction :type Input%20Action%20Object%20Reference :default "/Game/Input/Actions/IA_Jump.IA_Jump"))
  ;[1 1 1] Jump and Wall Jumping
  (:Started
    (if (Variables|Wall|GetIsWallSliding)
      (|WallJump)
      (else
        (Character|Jump)
        ;;[1 1 1] Jump Sound Effect
        (Audio|PlaySound2D "/Game/Audio/SFX/Player_Jump_Cue.Player_Jump_Cue" 1.0 1.0 0.0 0 0))))
  (:Canceled
    (Character|StopJumping :!label _label))
  (:Completed
    (goto _label)))

(event Input|EnhancedActionEvents|EnhancedInputActionIA_Move
  (params (ActionValue :type Vector%202D%20Structure) (ElapsedSeconds :type Float%20%28double-precision%29) (TriggeredSeconds :type Float%20%28double-precision%29) (InputAction :type Input%20Action%20Object%20Reference :default "/Game/Input/Actions/IA_Move.IA_Move"))
  ;[1 1 1] Movement
  ;;[1 1 1] Cannot Move When Damaged By Running Into Enemy
  (if (not (Variables|Stun|GetIsStunned))
    (Pawn|Input|AddMovementInput "1.000000,0.000000,0.000000" (.x ActionValue) false)
    (CallFunction|UpdateRotation (.x ActionValue))))

(event Input|EnhancedActionEvents|EnhancedInputActionIA_Shoot
  (params (ActionValue :type Boolean) (ElapsedSeconds :type Float%20%28double-precision%29) (TriggeredSeconds :type Float%20%28double-precision%29) (InputAction :type Input%20Action%20Object%20Reference :default "/Game/Input/Actions/IA_Shoot.IA_Shoot"))
  ;[1 1 1] Shooting and Energy Depletion
  (:Started
    (if (and (not (Variables|Stun|GetIsStunned)) (not (Variables|Slide|GetIsGroundSliding)))
      (Variables|Shooting|SetWasHitDuringCharge false)
      (Shooting|SpawnProjectile "/Game/Blueprints/Projectiles/Player/BP_PlayerProjectile_Regular.BP_PlayerProjectile_Regular_C")))
  (:Ongoing
    (Shooting|HandleChargeFlash ElapsedSeconds))
  (:Completed
    (if (and (not (Variables|Stun|GetIsStunned)) (not (Variables|Slide|GetIsGroundSliding)))
      (Shooting|TryChargedShot ElapsedSeconds)
      ;;[1 1 1] Deactivate's Charge Sound
      (Components|Activation|Deactivate (Variables|Default|GetChargeSound)))))

(event EventBeginPlay
  ;[1 1 1] Control Mapping
  (|CallParentFunction)
  ;;[1 1 1] Initiate Dynamic Material (Paralax Background Settings)
  (for (_array_element _array_index) (Components|GetChildrenComponents (Variables|Default|GetStaticBackground) false)
    (bind _aspaper_sprite_component (Utilities|Casting|CastToPaperSpriteComponent _array_element))
    (bind _returnvalue (Rendering|Material|CreateDynamicMaterialInstance _aspaper_sprite_component 0 0 "None" :!class /Script/Engine.PrimitiveComponent))
    (Utilities|Array|Add (Variables|Default|GetDynamicLayers) _returnvalue)
    (Rendering|Material|SetScalarParameterValue _returnvalue "ParalaxMultiplyer" (Utilities|Array|Get(acopy) (Variables|Default|GetParalaxMultipliers) _array_index) :!class /Script/Engine.MaterialInstanceDynamic)
    (Utilities|FlowControl|Sequence
      (:then_0
        (bind _asgm_action_platformer (Utilities|Casting|CastToGM_ActionPlatformer (Game|GetGameMode)))
        (Variables|Default|SetGMAction _asgm_action_platformer)
        (bind _asplayer_controller (Utilities|Casting|CastToPlayerController (Pawn|GetController)))
        (Input|AddMappingContext (PlayerController|LocalPlayerSubsystems|GetEnhancedInputLocalPlayerSubsystem _asplayer_controller) "/Game/Input/IMC_ActionGame.IMC_ActionGame" 0 "(bIgnoreAllPressedKeysUntilRelease=True,bForceImmediately=False,bNotifyUserSettings=False)"))
      (:then_1
        ;;[1 1 1] Jumping Friction Constant
        (Variables|Default|SetBaseLateralFriction (Variables|/Script/Engine.CharacterMovementComponent|GetFallingLateralFriction (Variables|Character|GetCharacterMovement)))
        ;;[1 1 1] Update Health After Respawn
        (Default|UpdateHealth (Variables|/Game/Widgets/WBP_HUD.WBP_HUD_C|GetWBP_HealthComponent (Variables|/Game/Blueprints/GM_ActionPlatformer.GM_ActionPlatformer_C|GetHudWidget (Variables|Default|GetGMAction))) (Variables|/Game/Blueprints/Components/BPC_Vitality.BPC_Vitality_C|GetCurrentHealth (Variables|Default|GetBPC_Vitality)))
        ;;[1 1 1] Set Camera Location Upon Spawn
        (Transformation|SetWorldLocation (Variables|Default|GetSpringArm) (Transformation|GetActorLocation) false false))
      (:then_2
        ;;[1 1 1] Player Respawn
        (EventDispatchers|BindEventtoDefeated (delegate Custom|OnDefeated))))))

(event Game|Damage|EventAnyDamage
  (params (Damage :type Float%20%28single-precision%29) (DamageType :type Damage%20Type%20Object%20Reference) (InstigatedBy :type Controller%20Object%20Reference) (DamageCauser :type Actor%20Object%20Reference))
  ;[1 1 1] Recieve Damage Logic (Touching Enemy Damage Knockback/ Animation Timing/ Update Health)
  (|CallParentFunction Damage DamageType InstigatedBy DamageCauser)
  (Default|UpdateHealth (Variables|/Game/Widgets/WBP_HUD.WBP_HUD_C|GetWBP_HealthComponent (Variables|/Game/Blueprints/GM_ActionPlatformer.GM_ActionPlatformer_C|GetHudWidget (Variables|Default|GetGMAction))) (Variables|/Game/Blueprints/Components/BPC_Vitality.BPC_Vitality_C|GetCurrentHealth (Variables|Default|GetBPC_Vitality)))
  (Components|Activation|Deactivate (Variables|Default|GetChargeSound))
  (Variables|Shooting|SetWasHitDuringCharge true)
  (if (not (Variables|/Game/Blueprints/Components/BPC_Vitality.BPC_Vitality_C|GetIsDefeated (Variables|Default|GetBPC_Vitality)))
    (CallFunction|TriggerInvincibility)
    (Audio|PlaySound2D "/Game/Audio/SFX/Impact_Flesh_Cue.Impact_Flesh_Cue" 1.0 1.0 0.0 0 0)
    (|Knockback DamageCauser)
    (else
      (Utilities|FlowControl|DoOnce false
        (:Completed
          (Audio|PlaySound2D "/Game/Audio/SFX/Player_Death_Cue.Player_Death_Cue" 1.0 1.0 0.0 0 0)
          (Class|PaperZDAnimInstance|JumptoNode (Variables|/Script/PaperZD.PaperZDAnimationComponent|GetAnimInstance (Variables|Default|GetAnimationComponent)) "JumpToDeath" "None"))))))

(event EventTick
  (params (DeltaSeconds :type Float%20%28single-precision%29))
  (|CallParentFunction DeltaSeconds)
  (WallSlide|TryWallSlide)
  (CallFunction|UpdateCameraPos))

(event EventOnWalkingOffLedge
  (params (PreviousFloorImpactNormal :type Vector%20%28by%20ref%29 :default "0, 0, 0") (PreviousFloorContactNormal :type Vector%20%28by%20ref%29 :default "0, 0, 0") (PreviousLocation :type Vector%20%28by%20ref%29 :default "0, 0, 0") (TimeDelta :type Float%20%28single-precision%29))
  ;[1 1 1] Slide Mechanics (Connect To Jump and Wall Jumping If Wanting To Slide - ACTIVATE OTHER DISABLED NODES ON GRAPH IF WANTING TO USE SLIDE)
  ;;[1 1 1] Cancel Slide Off Edge (Turn On If Using Slide)
  (CallFunction|CancelSlide))

(event EventOnLanded
  (params (Hit :type Hit%20Result%20Structure%20%28by%20ref%29))
  ;[1 1 1] Sound On Player Landing
  (Audio|PlaySound2D "/Game/Audio/SFX/Land_Player_Cue.Land_Player_Cue" 1.0 1.0 0.0 0 0))

(fn ConstructionScript
  (|CallParentFunction))

(fn UpdateRotation
  (params (Direction :type Float%20%28double-precision%29))
  ;[1 1 1] Check for Slide Value and Cant Turn While Sliding Logic
  (if (and (!= Direction 0.0) (not (Variables|Slide|GetIsGroundSliding)))
    (Pawn|SetControlRotation (Pawn|GetController) (select (>= Direction 0.0) (Math|Rotator|MakeRotator 0.0 0.0 0.0) (Math|Rotator|MakeRotator 0.0 0.0 1.8e+02)))))

(fn RestoreShotEnergy
  (params (ProjectileClass :type BP%20Player%20Projectile%20BASE%20Class%20Reference%20%28by%20ref%29))
  (Variables|Shooting|SetShotEnergy (Math|Integer|Min(Integer) (+ (Variables|Shooting|GetShotEnergy) (.Value (Utilities|Map|Find (Variables|Shooting|GetProjectileToEnergy) ProjectileClass))) (Variables|Shooting|GetMaxShotEnergy))))

(fn ToggleSpriteFlicker
  (Rendering|SetVisibility (Variables|Default|GetSprite) (not (Variables|/Script/Engine.SceneComponent|GetbVisible (Variables|Default|GetSprite))) false))

(fn SpawnProjectile
  (params (ProjectileClass :type BP%20Player%20Projectile%20BASE%20Class%20Reference))
  (bind _self self)
  (bind _shootpos (Variables|Default|GetShootPos))
  (bind _shootposwallslide (Variables|Default|GetShootPosWallSlide))
  (bind _iswallsliding (Variables|Wall|GetIsWallSliding))
  (bind _returnvalue (select _iswallsliding _shootposwallslide _shootpos))
  (bind _returnvalue_2 (Transformation|GetWorldTransform _returnvalue))
  ;[1 1 1] Energy Projectile Check (Checks If Enough Energy Is Avaliable For Shot Type)
  (if (>= (Variables|Shooting|GetShotEnergy) (.Value (Utilities|Map|Find (Variables|Shooting|GetProjectileToEnergy) ProjectileClass)))
    ;[1 1 1] Energy Projectile Cost (Takes The Cost From The Map List And Subracts Cost From Remaining Energy)
    (Variables|Shooting|SetShotEnergy (Math|Integer|Max(Integer) (- (Variables|Shooting|GetShotEnergy) (.Value (Utilities|Map|Find (Variables|Shooting|GetProjectileToEnergy) ProjectileClass)))))
    (Game|SpawnActorfromClass ProjectileClass (Math|Transform|MakeTransform (.location _returnvalue_2) (.rotation _returnvalue_2) "1.000000,1.000000,1.000000") "AlwaysSpawn" "MultiplyWithRoot" _self _self)
    (CallFunction|TriggerShootAnim)
    (Audio|PlaySound2D (select (== ProjectileClass "/Game/Blueprints/Projectiles/Player/BP_PlayerProjectile_FullCharge.BP_PlayerProjectile_FullCharge_C") "/Game/Audio/SFX/Fire_ChargedShot.Fire_ChargedShot" "/Game/Audio/SFX/Shot_Regular_Cue.Shot_Regular_Cue") 1.0 1.0 0.0 0 0)))

(fn TryChargedShot
  (params (ElapsedTime :type Float%20%28double-precision%29))
  ;[1 1 1] Charge Shot Cancel If Hit
  (if (not (Variables|Shooting|GetWasHitDuringCharge))
    ;[1 1 1] Time For Partical Charge Shot
    (if (>= ElapsedTime (Variables|Shooting|GetPartialChargeTime))
      ;[1 1 1] Time For Full Charge Shot
      (if (>= ElapsedTime (Variables|Shooting|GetFullChargeTime))
        (Shooting|SpawnProjectile "/Game/Blueprints/Projectiles/Player/BP_PlayerProjectile_FullCharge.BP_PlayerProjectile_FullCharge_C")
        (else
          (Shooting|SpawnProjectile "/Game/Blueprints/Projectiles/Player/BP_PlayerProjectile_PartialCharge.BP_PlayerProjectile_PartialCharge_C"))))))

(fn HandleChargeFlash
  (params (Elapsed :type Float%20%28double-precision%29))
  (if (and (>= Elapsed (Variables|Shooting|GetPartialChargeTime)) (not (Variables|Shooting|GetWasHitDuringCharge)))
    (Variables|Shooting|SetChargeFlashTimer (+ (Variables|Shooting|GetChargeFlashTimer) (Utilities|Time|GetWorldDeltaSeconds)))
    (if (>= (Variables|Shooting|GetChargeFlashTimer) (Variables|Shooting|GetChargeFlashInterval))
      ;[1 1 1] Fully Charged Sound Effect
      (Components|Activation|Activate (Variables|Default|GetChargeSound) false)
      (Variables|Shooting|SetChargeFlashTimer 0.0)
      (CallFunction|TriggerFlash 5.0 (select (>= Elapsed (Variables|Shooting|GetFullChargeTime)) "(R=1.000000,G=0.029851,B=0.079611,A=1.000000)" "(R=1.000000,G=1.000000,B=1.000000,A=1.000000)")))
    (else
      (Variables|Shooting|SetChargeFlashTimer 0.0))))

(fn TryWallSlide
  (bind _returnvalue (Transformation|GetActorLocation))
  ;[1 1 1] Wall Grab Velocity And Direction (Sets Velocity Player Is Falling Before Grabs The Wall and Direction Player Is Facing)
  (if (and (|IsDecending) (|IsHoldingTowardsWall))
    (bind _returnvalue_2 (Collision|LineTraceForObjects _returnvalue (+ _returnvalue (* (Transformation|GetActorForwardVector) (Variables|Wall|GetWallTraceLength))) (Utilities|Array|MakeArray "ObjectTypeQuery1") false 0 "ForOneFrame"))
    (if _returnvalue_2
      (Variables|Wall|SetIsWallSliding true)
      ;[1 1 1] Wall Slide Movement Speed
      (Variables|/Script/Engine.MovementComponent|SetVelocity (Variables|Character|GetCharacterMovement) (Math|Vector|MakeVector (.x (Variables|/Script/Engine.MovementComponent|GetVelocity (Variables|Character|GetCharacterMovement))) (.y (Variables|/Script/Engine.MovementComponent|GetVelocity (Variables|Character|GetCharacterMovement))) (Math|Float|Max(Float) (.z (Variables|/Script/Engine.MovementComponent|GetVelocity (Variables|Character|GetCharacterMovement))) (Variables|Wall|GetWallSlideSpeed))))
      (else
        (Variables|Wall|SetIsWallSliding false)))
    (else
      (Variables|Wall|SetIsWallSliding false))))

(fn TryCancelSlide
  (if (and (Variables|Slide|GetIsGroundSliding) (< (* (.x (Transformation|GetActorForwardVector)) (.x (Input|EnhancedActionValues|GetIA_Move))) 0.0))
    (CallFunction|CancelSlide)))

(fn UpdateCameraPos
  (if (not (Variables|/Game/Blueprints/Components/BPC_Vitality.BPC_Vitality_C|GetIsDefeated (Variables|Default|GetBPC_Vitality)))
    (Utilities|IsValid (Variables|Default|GetOverlappingRestrictor)
      (:Is%20Valid
        ;[1 1 1] Snaps to Camera Restrictor
        (Transformation|SetWorldLocation (Variables|Default|GetSpringArm) (Math|Interpolation|VInterpTo (Transformation|GetWorldLocation (Variables|Default|GetSpringArm)) (Transformation|GetActorLocation (Variables|Default|GetOverlappingRestrictor)) (Utilities|Time|GetWorldDeltaSeconds) (Variables|Default|GetCameraInterpSpeed)) false false))
      (:Is%20Not%20Valid
        ;[1 1 1] Snaps Away From Camera Restrictor
        (Transformation|SetWorldLocation (Variables|Default|GetSpringArm) (Math|Interpolation|VInterpTo (Transformation|GetWorldLocation (Variables|Default|GetSpringArm)) (+ (Transformation|GetActorLocation) (Math|Vector|MakeVector 0.0 0.0 (Variables|Default|GetCameraOffsetHeight))) (Utilities|Time|GetWorldDeltaSeconds) (Variables|Default|GetCameraInterpSpeed)) false false)))))