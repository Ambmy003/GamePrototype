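; BP_Checkpoint is a checkpoint prop for an action platformer, shown as an obelisk flipbook.
; The first time BP_Player overlaps its Box, it sets itself as the ActiveCheckpoint on GM_ActionPlatformer, cached at BeginPlay.
; It then plays the activation flipbook and, after a fixed delay, switches to the active one, shifting the obelisk's relative position for each.
; A DoOnce keeps activation from repeating on later overlaps.
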(event OnComponentBeginOverlap(Box)
  (params (OverlappedComponent :type Primitive%20Component%20Object%20Reference) (OtherActor :type Actor%20Object%20Reference) (OtherComp :type Primitive%20Component%20Object%20Reference) (OtherBodyIndex :type Integer) (bFromSweep :type Boolean) (SweepResult :type Hit%20Result%20Structure%20%28by%20ref%29))
  (Utilities|Casting|CastToBP_Player OtherActor)
  (Utilities|FlowControl|DoOnce false
    (:Completed
      (Variables|/Game/Blueprints/GM_ActionPlatformer.GM_ActionPlatformer_C|SetActiveCheckpoint (Variables|Default|GetGMAction) self)
      ;[1 1 1] Updates Relative Location and Sprite Of The Checkpoint
      (Transformation|SetRelativeLocation (Variables|Default|GetObelisk) "0.000000,0.000000,17.500000" false false)
      (Sprite|SetFlipbook (Variables|Default|GetObelisk) "/Game/PaperAssets/Environment/Obelisk/Obelisk_Activation.Obelisk_Activation")
      (Utilities|FlowControl|Delay 1.35)
      (Transformation|SetRelativeLocation (Variables|Default|GetObelisk) "0.000000,0.000000,-70.000000" false false)
      (Sprite|SetFlipbook (Variables|Default|GetObelisk) "/Game/PaperAssets/Environment/Obelisk/Obelisk_Active.Obelisk_Active"))))

(event EventBeginPlay
  (bind _asgm_action_platformer (Utilities|Casting|CastToGM_ActionPlatformer (Game|GetGameMode)))
  (Variables|Default|SetGMAction _asgm_action_platformer))

(event Collision|EventActorBeginOverlap
  (params (OtherActor :type Actor%20Object%20Reference)))

(event EventTick
  (params (DeltaSeconds :type Float%20%28single-precision%29)))

(fn ConstructionScript)