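; Boss wall prop that slides to a new position when play begins, provided the boss is not defeated.
; BeginPlay caches the world locations of the wall component and a Scene marker, and CloseWall fetches the first BP_Boss in the level.
; A timeline then lerps the whole actor between those two locations without sweeping.
; The defeated check runs only once, and overlap and tick events are empty.
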(event Custom|CloseWall
  (bind _outactors (Actor|GetAllActorsOfClass "/Game/BossFight/BP_Boss.BP_Boss_C"))
  (Variables|Default|SetBoss (Utilities|Array|Get(acopy) _outactors)))

(event EventBeginPlay
  (Variables|Default|SetBossWallTwoLocation (Transformation|GetWorldLocation (Variables|Default|GetBossWallTwo)))
  (Variables|Default|SetBossWallTwoMovement (Transformation|GetWorldLocation (Variables|Default|GetScene)))
  (CallFunction|CloseWall)
  (if (not (Variables|/Game/Blueprints/Characters/Enemies/BP_Enemy_BASE.BP_Enemy_BASE_C|GetIsDefeated (Variables|Default|GetBoss)))
    (bind _alpha (Timeline|PlayAnim Play)
      (:Update
        (Transformation|SetActorLocation (Math|Vector|Lerp(Vector) (Variables|Default|GetBossWallTwoLocation) (Variables|Default|GetBossWallTwoMovement) _alpha) false false)))))

(event Collision|EventActorBeginOverlap
  (params (OtherActor :type Actor%20Object%20Reference)))

(event EventTick
  (params (DeltaSeconds :type Float%20%28single-precision%29)))

(fn ConstructionScript)