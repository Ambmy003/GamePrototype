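; BP_BossWallOne is a prop wall that moves into a new position after something enters its trigger box.
; BeginPlay caches the world locations of the BossWall component and a Scene component as start and end points.
; Box overlap waits briefly, then plays the MoveAnim timeline, lerping the whole actor between those points without sweep.
; The overlap has no filter on the overlapping actor.
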(event OnComponentBeginOverlap(Box)
  (params (OverlappedComponent :type Primitive%20Component%20Object%20Reference) (OtherActor :type Actor%20Object%20Reference) (OtherComp :type Primitive%20Component%20Object%20Reference) (OtherBodyIndex :type Integer) (bFromSweep :type Boolean) (SweepResult :type Hit%20Result%20Structure%20%28by%20ref%29))
  (Utilities|FlowControl|Delay 1.0)
  (bind _alpha (Timeline|MoveAnim Play)
    (:Update
      (Transformation|SetActorLocation (Math|Vector|Lerp(Vector) (Variables|Default|GetBossWallOneLocation) (Variables|Default|GetBossWallMovement) _alpha) false false))))

(event EventBeginPlay
  (Variables|Default|SetBossWallOneLocation (Transformation|GetWorldLocation (Variables|Default|GetBossWall)))
  (Variables|Default|SetBossWallMovement (Transformation|GetWorldLocation (Variables|Default|GetScene))))

(event Collision|EventActorBeginOverlap
  (params (OtherActor :type Actor%20Object%20Reference)))

(event EventTick
  (params (DeltaSeconds :type Float%20%28single-precision%29)))

(fn ConstructionScript)