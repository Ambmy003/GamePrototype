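; Boss enemy with a water-ball shot and left/right dashes, using a PaperZD-style animation component.
; Dash events jump to the dash animation and use timelines to lerp X and Z toward marker positions cached at BeginPlay, calling the end dispatcher every update.
; Player overlap with AggroRange creates the health widget, refreshed each Tick from BPCVitality.
; Shooting plays an override animation; separate functions handle projectile spawning and hitbox damage.
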(event OnComponentBeginOverlap(AggroRange)
  (params (OverlappedComponent :type Primitive%20Component%20Object%20Reference) (OtherActor :type Actor%20Object%20Reference) (OtherComp :type Primitive%20Component%20Object%20Reference) (OtherBodyIndex :type Integer) (bFromSweep :type Boolean) (SweepResult :type Hit%20Result%20Structure%20%28by%20ref%29))
  (Utilities|Casting|CastToBP_Player OtherActor)
  (Variables|Default|SetPlayerInRange true)
  ;[1 1 1] Boss Health Widget
  (bind _returnvalue (UserInterface|CreateWidget "/Game/BossFight/WBP_BossFightHealth.WBP_BossFightHealth_C"))
  (UserInterface|Viewport|AddtoViewport _returnvalue 0)
  (Variables|Default|SetHeathUI _returnvalue))

(event Custom|DashAttack
  ;[1 1 1] Boss Dash Attack Left
  (Utilities|FlowControl|Delay 0.1)
  (Class|PaperZDAnimInstance|JumptoNode (Variables|/Script/PaperZD.PaperZDAnimationComponent|GetAnimInstance (Variables|Default|GetAnimationComponent)) "JumpToDash" "None")
  (bind _alpha (Timeline|MoveAnimLeft Play)
    (:Update
      (Transformation|SetActorLocation (Math|Vector|MakeVector (.x (Math|Vector|Lerp(Vector) (Transformation|GetWorldLocation (Variables|Default|GetCapsuleComponent)) (Variables|Default|GetWorldLeftPos) _alpha)) 0.0 (.z (Math|Vector|Lerp(Vector) (Transformation|GetWorldLocation (Variables|Default|GetCapsuleComponent)) (Variables|Default|GetWorldLeftPos) _alpha))) false false)
      (Default|CallOnDashAttackEnd))))

(event Custom|ShootAttack
  (CallFunction|ShootWaterBall)
  (Utilities|FlowControl|Delay 0.0)
  (Default|CallOnShootAttackEnd))

(event Custom|DashAttackRight
  (Utilities|FlowControl|Delay 0.1)
  (Class|PaperZDAnimInstance|JumptoNode (Variables|/Script/PaperZD.PaperZDAnimationComponent|GetAnimInstance (Variables|Default|GetAnimationComponent)) "JumpToDash" "None")
  (bind _alpha (Timeline|MoveAnimRight Play)
    (:Update
      (Transformation|SetActorLocation (Math|Vector|MakeVector (.x (Math|Vector|Lerp(Vector) (Transformation|GetWorldLocation (Variables|Default|GetCapsuleComponent)) (Variables|Default|GetWorldRightPos) _alpha)) 0.0 (.z (Math|Vector|Lerp(Vector) (Transformation|GetWorldLocation (Variables|Default|GetCapsuleComponent)) (Variables|Default|GetWorldRightPos) _alpha))) false false)
      (Default|CallOnDashAttackEnd))))

(event EventBeginPlay
  (|CallParentFunction)
  (Variables|Default|SetWorldRightPos (Transformation|GetWorldLocation (Variables|Default|GetRightPos)))
  (Variables|Default|SetWorldLeftPos (Transformation|GetWorldLocation (Variables|Default|GetLeftPos)))
  (Components|Timeline|SetPlayRate (Variables|Default|GetMoveAnimLeft) (Variables|Default|GetMovePlayRateLeft))
  (Components|Timeline|SetPlayRate (Variables|Default|GetMoveAnimRight) (Variables|Default|GetMovePlayRateRight)))

(event Collision|EventActorBeginOverlap
  (params (OtherActor :type Actor%20Object%20Reference))
  (|CallParentFunction OtherActor) ; This node is disabled and will not be called.\nDrag off pins to build functionality.
)

(event EventTick
  (params (DeltaSeconds :type Float%20%28single-precision%29))
  (|CallParentFunction DeltaSeconds)
  (if (Variables|Default|GetPlayerInRange)
    (CallFunction|BossHealth)))

(fn ConstructionScript
  (|CallParentFunction))

(fn BossHealth
  (Progress|SetPercent (Variables|/Game/BossFight/WBP_BossFightHealth.WBP_BossFightHealth_C|GetBossHealthBar (Variables|Default|GetHeathUI)) (/ (Variables|/Game/Blueprints/Components/BPC_Vitality.BPC_Vitality_C|GetCurrentHealth (Variables|Default|GetBPC_Vitality)) (Variables|/Game/Blueprints/Components/BPC_Vitality.BPC_Vitality_C|GetMaxHealth (Variables|Default|GetBPC_Vitality)))))

(fn HitCheck
  (for _array_element (Collision|GetOverlappingActors (Variables|Default|GetAttackHitBox) "/Game/Blueprints/Projectiles/BP_Projectile_BASE.BP_Projectile_BASE_C" :!class /Script/Engine.PrimitiveComponent)
    (if (!= _array_element self)
      (Game|Damage|ApplyDamage _array_element (Variables|Default|GetAttackDamage) 0 0))))

(fn SpawnProjectile
  (bind _shotpos (Variables|Default|GetShotPos))
  (Game|SpawnActorfromClass "/Game/Blueprints/Projectiles/Enemy/BP_EnemyProjectile_Boss.BP_EnemyProjectile_Boss_C" (Math|Transform|MakeTransform (Transformation|GetWorldLocation _shotpos) (Transformation|GetWorldRotation _shotpos) "1.000000,1.000000,1.000000") "AlwaysSpawn" "MultiplyWithRoot" 0 0)
  (Audio|PlaySoundatLocation "/Game/Audio/SFX/Water_Shot_Cue.Water_Shot_Cue" (Transformation|GetActorLocation) "0, 0, 0" 1.0 1.0 0.0 0 0 0 0))

(fn ShootWaterBall
  (Class|PaperZDAnimInstance|PlayAnimationOverride (Variables|/Script/PaperZD.PaperZDAnimationComponent|GetAnimInstance (Variables|Default|GetAnimationComponent)) "/Game/BossFight/AnimSequences/AttackShot.AttackShot" "DefaultSlot" 1.0 0.0))